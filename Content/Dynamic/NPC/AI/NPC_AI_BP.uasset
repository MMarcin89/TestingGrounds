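; AI controller for guard NPCs that detects player-controlled targets and passes them to a behavior tree.
; On BeginPlay it sets up the PatrolData blackboard and runs GuardBehavior.
; Perception updates filter on the actor's instigator being player-controlled, then write the enemy and its location to the blackboard.
; Losing the stimulus clears only the enemy key, so the last sensed location remains stored.
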(event OnTargetPerceptionUpdated(AIPerception)
  (params (Actor :type Actor%20Object%20Reference) (Stimulus :type AI%20Stimulus%20Structure))
  (bind _blackboardcomponent (Variables|Default|GetBlackboardComponent))
  (bind _enemykey (Variables|Default|GetEnemyKey))
  (if (Pawn|IsPlayerControlled (Variables|/Script/Engine.Actor|GetInstigator Actor))
    (if (.bSuccessfullySensed (Utilities|Struct|BreakAIStimulus Stimulus))
      (AI|Components|Blackboard|SetValueasObject _blackboardcomponent _enemykey Actor)
      (AI|Components|Blackboard|SetValueasVector _blackboardcomponent (Variables|Default|GetEnemyLocation) (Transformation|GetActorLocation Actor))
      (else
        (AI|Components|Blackboard|ClearValue _blackboardcomponent _enemykey)))))

(event EventBeginPlay
  (bind _blackboardcomponent (Class|AIController|UseBlackboard "/Game/Dynamic/NPC/AI/PatrolData.PatrolData"))
  (AI|RunBehaviorTree "/Game/Dynamic/NPC/AI/GuardBehavior.GuardBehavior")
  (Variables|Default|SetBlackboardComponent _blackboardcomponent))

(fn ConstructionScript)